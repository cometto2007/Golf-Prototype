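; AccelerationPlatform is an actor that launches the golf ball when it overlaps the platform.
; On overlap it casts to GolfBall and calls DoImpulse with a fixed strength.
; If the Direction actor is set, the impulse points from the ball toward that actor and passes NewVelocity as true.
; Otherwise it follows the ball camera's forward vector with NewVelocity false.
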(event EventBeginPlay)

(event Collision|EventActorBeginOverlap
  (params (OtherActor :type Actor%20Object%20Reference))
  (bind _asgolf_ball (Utilities|Casting|CastToGolfBall OtherActor))
  (if (!= (Variables|Default|GetDirection) 0)
    (Default|DoImpulse _asgolf_ball 2.5e+05 (Math|Vector|Normalize (- (Transformation|GetActorLocation (Variables|Default|GetDirection)) (Transformation|GetActorLocation _asgolf_ball))) true)
    (else
      (Default|DoImpulse _asgolf_ball 2.5e+05 (Math|Vector|GetForwardVector (Variables|/Game/Prototype/Blueprint/Pawn/GolfBall.GolfBall_C|GetCamera _asgolf_ball)) false))))

(event EventTick
  (params (DeltaSeconds :type Float%20%28single-precision%29)))

(fn ConstructionScript)