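; EnemyCharger is a prototype enemy pawn that charges at the player's golf ball and can be killed by projectiles.
; When its PawnSensing component sees a GolfBall pawn, it uses AI MoveTo to chase that actor.
; Each overlapping Projectile removes a fixed amount of Health and spawns an explosion effect at the projectile's sphere.
; Tick polls Health and destroys the actor once it is depleted.
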(event OnSeePawn(PawnSensing)
  (params (Pawn :type Pawn%20Object%20Reference))
  (bind _asgolf_ball (Utilities|Casting|CastToGolfBall Pawn))
  (AI|AIMoveTo self "0, 0, 0" _asgolf_ball 5.0 false))

(event EventBeginPlay)

(event Collision|EventActorBeginOverlap
  (params (OtherActor :type Actor%20Object%20Reference))
  (bind _asprojectile (Utilities|Casting|CastToProjectile OtherActor))
  (Variables|Default|Sethealth (- (Variables|Default|Gethealth) 5e+01))
  (Effects|SpawnEmitteratLocation "/Game/Prototype/StarterContent/P_Explosion.P_Explosion" (Transformation|GetWorldLocation (Variables|/Game/Prototype/Blueprint/Actors/Projectile.Projectile_C|GetSphere _asprojectile)) "0, 0, 0" "3.000000,3.000000,3.000000"))

(event EventTick
  (params (DeltaSeconds :type Float%20%28single-precision%29))
  (if (<= (Variables|Default|Gethealth) 0.0)
    (Actor|DestroyActor)))

(fn ConstructionScript)