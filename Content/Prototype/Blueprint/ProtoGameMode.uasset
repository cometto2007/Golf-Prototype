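; ProtoGameMode is a prototype game mode that sets up the in-game HUD and keeps a running count of seconds.
; On BeginPlay it creates the HUD widget for the first player controller and adds it to the viewport, except in the MainMenu level.
; Tick feeds a one-second Delay, which ignores re-triggers while pending, so the Seconds counter increments roughly once per second.
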(event EventTick
  (params (DeltaSeconds :type Float%20%28single-precision%29))
  ;[1 1 1] Keep track of the seconds
  (Utilities|FlowControl|Delay 1.0)
  (Variables|Default|SetSeconds (+ (Variables|Default|GetSeconds) 1)))

(event EventBeginPlay
  ;[1 1 1] Create HUD
  (bind _returnvalue (Game|GetCurrentLevelName true))
  (if (Utilities|Enum|NotEqual(Enum) _returnvalue "MainMenu")
    (bind _returnvalue_2 (UserInterface|CreateWidget "/Game/Prototype/Blueprint/UI/HUD.HUD_C" (Game|GetPlayerController 0)))
    (UserInterface|Viewport|AddtoViewport _returnvalue_2 0)))

(fn ConstructionScript)